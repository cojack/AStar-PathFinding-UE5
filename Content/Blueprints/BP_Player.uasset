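; Player blueprint for a pathfinding grid: shows the cursor and lets the mouse edit the grid.
; On BeginPlay it adds the WBP_PathFinding widget and centers itself above the grid using cell count and size.
; Left and right clicks pass the deprojected mouse position to PathFinding to toggle walls and begin/end cells.
; Tick resizes the orthographic camera width to fit the whole grid plus margin at the viewport's aspect ratio.
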(event EventBeginPlay
  (bind _pathfinding (Variables|Default|GetPathFinding))
  (bind _cellsize (Variables|/Script/AStarPathFinding.PathFinding|GetCellSize _pathfinding))
  (bind _returnvalue (/ _cellsize 2.0))
  (Variables|/Script/Engine.PlayerController|SetbShowMouseCursor (Game|GetPlayerController 0) true)
  (bind _returnvalue_2 (UserInterface|CreateWidget "/Game/Blueprints/WBP_PathFinding.WBP_PathFinding_C" 0 self))
  (UserInterface|Viewport|AddtoViewport _returnvalue_2 0)
  (Transformation|SetActorLocation (Math|Vector|MakeVector (- (/ (* (Variables|/Script/AStarPathFinding.PathFinding|GetHorizontalCells _pathfinding) _cellsize) 2.0) _returnvalue) (* (- (/ (* _cellsize (Variables|/Script/AStarPathFinding.PathFinding|GetVerticalCells _pathfinding)) 2.0) _returnvalue) -1.0) 5e+02) false false))

(event EventTick
  (params (DeltaSeconds :type Float%20%28single-precision%29))
  (bind _returnvalue (Viewport|GetViewportSize))
  (bind _pathfinding (Variables|Default|GetPathFinding))
  (bind _pathfinding_2 (Variables|Default|GetPathFinding))
  (bind _cellsize (Variables|/Script/AStarPathFinding.PathFinding|GetCellSize _pathfinding_2))
  (bind _cellsize_2 (Variables|/Script/AStarPathFinding.PathFinding|GetCellSize _pathfinding))
  (Class|CameraComponent|SetOrthoWidth (Variables|Default|GetCamera) (Math|Float|Max(Float) (+ (* (Variables|/Script/AStarPathFinding.PathFinding|GetHorizontalCells _pathfinding_2) _cellsize) _cellsize) (* (+ (* (Variables|/Script/AStarPathFinding.PathFinding|GetVerticalCells _pathfinding) _cellsize_2) _cellsize_2) (/ (.x _returnvalue) (.y _returnvalue))))))

(event Input|MouseEvents|LeftMouseButton
  (params (Key :type Key%20Structure))
  (:Pressed
    (Class|PathFinding|ToggleWall (Variables|Default|GetPathFinding) (.WorldLocation (Game|Player|ConvertMouseLocationToWorldSpace (Game|GetPlayerController 0))))))

(event Input|MouseEvents|RightMouseButton
  (params (Key :type Key%20Structure))
  (:Pressed
    (Class|PathFinding|ToggleBeginEnd (Variables|Default|GetPathFinding) (.WorldLocation (Game|Player|ConvertMouseLocationToWorldSpace (Game|GetPlayerController 0))))))

(fn ConstructionScript)